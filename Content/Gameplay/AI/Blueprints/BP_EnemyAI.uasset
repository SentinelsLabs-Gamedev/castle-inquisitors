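; BP_EnemyAI is an enemy that spots the player character and attacks it in melee.
; Pawn sensing sets a "hasSeenPlayer?" blackboard flag, and a retriggerable delay clears it shortly after the last sighting.
; AttackPlayer sphere-traces ahead of the enemy and, on hitting the player character, plays an attack montage and applies damage.
; The attack trace still draws debug shapes.
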(event `self.PawnSensingComponent.OnSeePawn`
  (params (Pawn :type "Pawn Object Reference"))
  (bind _returnvalue (`AIBlueprintHelperLibrary.GetBlackboard` (`AIBlueprintHelperLibrary.GetAIController` self)))
  (cast `CastleInquisitorsCharacter` Pawn)
  (`BlackboardComponent.SetValueAsBool` _returnvalue "hasSeenPlayer?" true)
  (`KismetSystemLibrary.RetriggerableDelay` 1.5)
  (`BlackboardComponent.SetValueAsBool` _returnvalue "hasSeenPlayer?" false))

(event `Attack Player`
  (bind _returnvalue (`self.K2_GetActorLocation`))
  (bind (_outhit _returnvalue_2) (`KismetSystemLibrary.SphereTraceSingleForObjects` :`Start` _returnvalue :`End` (+ _returnvalue (* (`KismetMathLibrary.GetForwardVector` (`self.K2_GetActorRotation`)) 250.0)) :`Radius` 120.0 :`ObjectTypes` (`|MakeArray` "ObjectTypeQuery3" :!type "EObjectTypeQuery Enum") :`DrawDebugType` "ForDuration"))
  (if _returnvalue_2
    (bind (_bblockinghit _binitialoverlap _time _distance _location _impactpoint _normal _impactnormal _physmat _hitactor) (`GameplayStatics.BreakHitResult` _outhit))
    (cast `CastleInquisitorsCharacter` _hitactor)
    (`self.PlayAnimMontage` "/Game/Gameplay/AI/Animations/AM_EnemyAIAttack.AM_EnemyAIAttack")
    (`GameplayStatics.ApplyDamage` _hitactor 10.0)))

(fn `UserConstructionScript`)