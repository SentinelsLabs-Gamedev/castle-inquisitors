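; BP_TreesGrid is a construction-time grid builder that lays out copies of one static mesh, presumably trees given the asset name.
; The Construction Script runs nested loops over X and Y, adding an instance to the TileStaticMesh component at each cell.
; Spacing comes from the mesh's local bounds, rounded up to whole units, so tiles sit edge to edge or nearly so.
; The event graph holds no logic.
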(event `self.ReceiveBeginPlay`)

(fn `UserConstructionScript`
  (bind (_min _max) (`StaticMeshComponent.GetLocalBounds` (`self.TileStaticMesh`)))
  (for _index (range (+ (`self.X`) 1))
    (for _index_2 (range (+ (`self.Y`) 1))
      (`InstancedStaticMeshComponent.AddInstance` (`self.TileStaticMesh`) (`KismetMathLibrary.MakeTransform` (`KismetMathLibrary.MakeVector` (`KismetMathLibrary.Conv_Int64ToDouble` (* _index (`KismetMathLibrary.FCeil64` (- (.x _max) (.x _min))))) (`KismetMathLibrary.Conv_IntToDouble` (* _index_2 (`KismetMathLibrary.FCeil64` (- (.y _max) (.y _min))))))) false))))